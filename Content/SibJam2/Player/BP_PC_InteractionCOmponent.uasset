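; Player controller interaction component that lets the player look at and interact with objects in the world.
; Every tick it line-traces on the Visibility channel from the controller's eye viewpoint up to a max range.
; Hit actors implementing SGJ_Interactable become the current target and supply look-on text to an on-screen widget, both cleared otherwise.
; Interact sends an interface message to that target, passing the owning controller.
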(event `self.ReceiveBeginPlay`
  (bind _returnvalue (`|CreateWidget` "/Game/SibJam2/Interaction/W_Interaction.W_Interaction_C"))
  (bind _output_get (set `self.InteractionWidget` _returnvalue))
  (`UserWidget.AddToViewport` _output_get 0))

(event `self.ReceiveTick`
  (params (DeltaSeconds :type "Float (single-precision)"))
  (`self.ActorUnderSight`))

(event `ActorUnderSight`
  (bind _interactionwidget (`self.InteractionWidget`))
  (bind _asplayer_controller (cast `PlayerController` (`self.GetOwner`)))
  (bind (_outlocation _outrotation) (`Actor.GetActorEyesViewPoint` _asplayer_controller))
  (bind (_outhit _returnvalue) (`KismetSystemLibrary.LineTraceSingle` _outlocation (+ _outlocation (* (`KismetMathLibrary.GetForwardVector` _outrotation) (`self.MaxRange`))) "TraceTypeQuery1"))
  (if _returnvalue
    (bind (_bblockinghit _binitialoverlap _time _distance _location _impactpoint _normal _impactnormal _physmat _hitactor) (`GameplayStatics.BreakHitResult` _outhit))
    (if (`KismetSystemLibrary.DoesImplementInterface` _hitactor "/Script/SibJam2.SGJ_Interactable")
      (bind _returnvalue_2 (message `SGJ_Interactable.GetLookOnMessage` _hitactor))
      (`/Game/SibJam2/Interaction/W_Interaction.SetInteractionMessage` _interactionwidget _returnvalue_2)
      (set `self.InteractionTarget` _hitactor)
      (else
        (`/Game/SibJam2/Interaction/W_Interaction.SetInteractionMessage` _interactionwidget "" :!label _label)
        (set `self.InteractionTarget` null)))
    (else
      (goto _label))))

(event `Interact`
  (message `SGJ_Interactable.InteractWith` (`self.InteractionTarget`) (`self.GetOwner`)))