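; BP_RatSpawner is a placed spawner that periodically fills an area with BP_Rat actors.
; A looping timer with a randomized start delay spawns a rat at a random XY point inside the Box extent, at the spawner's height with random yaw.
; Each rat is owned by the spawner and added to Rats.
; Spawning continues while that array's length is at most MaxRats, and nothing here removes entries.
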(event `self.ReceiveBeginPlay`
  (`KismetSystemLibrary.K2_SetTimerDelegate` (delegate `SpawnRat`) 5.0 true false 0.0 5.0))

(event `SpawnRat`
  (bind (_returnvalue_roll _returnvalue_pitch _returnvalue_yaw) (`KismetMathLibrary.BreakRotator` (`KismetMathLibrary.RandomRotator` false)))
  (bind (_returnvalue_x _returnvalue_y _returnvalue_z) (`KismetMathLibrary.BreakVector` (`self.K2_GetActorLocation`)))
  (bind (_returnvalue_x_2 _returnvalue_y_2) (`KismetMathLibrary.BreakVector` (`KismetMathLibrary.RandomPointInBoundingBox` (`self.K2_GetActorLocation`) (`BoxComponent.GetScaledBoxExtent` (`self.Box`)))))
  (if (>= (`self.MaxRats`) (`BlueprintSetLibrary.Set_Length` (`self.Rats`)))
    (bind _returnvalue (`|SpawnActorFromClass` "/Game/SibJam2/Blueprints/Characters/Rat/BP_Rat.BP_Rat_C" (`KismetMathLibrary.MakeTransform` (`KismetMathLibrary.MakeVector` _returnvalue_x_2 _returnvalue_y_2 _returnvalue_z) (`KismetMathLibrary.MakeRotator` 0.0 0.0 _returnvalue_yaw)) "AdjustIfPossibleButDontSpawnIfColliding" "MultiplyWithRoot" self null))
    (`BlueprintSetLibrary.Set_Add` (`self.Rats`) _returnvalue)))

(fn `UserConstructionScript`)