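; BPC_Player is the player controller that handles the interact input for BP_Player.
; IA_Interact triggers InteractionComponent on a valid target, otherwise it releases whatever the pawn's HoldComponent controls.
; Release re-enables the held actor's collision, then only for a BP_Hold_Log turns on mesh physics and clears the hold without destroying it.
; Other held actors regain collision but stay held, because the failed log cast ends the chain.
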(event `EnhancedInput|/Game/SibJam2/Blueprints/Characters/Player/Assets/IA_Interact`
  (params (ActionValue :type Boolean) (ElapsedSeconds :type "Float (double-precision)") (TriggeredSeconds :type "Float (double-precision)") (InputAction :type "InputAction Object Reference" :default "/Game/SibJam2/Blueprints/Characters/Player/Assets/IA_Interact.IA_Interact"))
  (bind _holdcomponent (`/Game/SibJam2/Blueprints/Characters/Player/BP_Player.HoldComponent` (cast `/Game/SibJam2/Blueprints/Characters/Player/BP_Player` (`self.K2_GetPawn`) :!pure true)))
  (bind _controlledactor (`SGJ_Player_HoldComponent.ControlledActor` _holdcomponent))
  (:`Triggered`
    (`/Engine/EditorBlueprintResources/StandardMacros.IsValid` (`/Game/SibJam2/Player/BP_PC_InteractionCOmponent.InteractionTarget` (`self.InteractionComponent`))
      (:`Is Valid`
        (`/Game/SibJam2/Player/BP_PC_InteractionCOmponent.Interact` (`self.InteractionComponent`)))
      (:`Is Not Valid`
        (`/Engine/EditorBlueprintResources/StandardMacros.IsValid` _controlledactor
          (:`Is Valid`
            (`self.SetActorEnableCollision` _controlledactor true)
            (bind _asbp_hold_log (cast `/Game/SibJam2/Objects/Hold/BP_Hold_Log` _controlledactor))
            (`PrimitiveComponent.SetSimulatePhysics` (`/Game/SibJam2/Objects/Hold/BP_Hold_Log.Mesh` _asbp_hold_log) true)
            (`SGJ_Player_HoldComponent.SetNewControlledActor` _holdcomponent null false)))))))

(fn `UserConstructionScript`)