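; BPC_Bot is the AI controller for bot characters, responsible for setting up and feeding their blackboard.
; On BeginPlay it initializes BB_Bot, then stores its MoveTarget object and the first player's character as blackboard keys.
; Two events let other logic write the target count and the bot's state enum to the blackboard.
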(event `SetTargetCountToBlackboard`
  (params (NewTargetCount :type Integer))
  (`BlackboardComponent.SetValueAsInt` (`AIBlueprintHelperLibrary.GetBlackboard` null) (`self.TargetCountKey`) NewTargetCount))

(event `SetStateToBlackboard`
  (params (State :type "/Game/SibJam2/Blueprints/Characters/Bot/Enum_BotStates Enum" :default "NewEnumerator0"))
  (`BlackboardComponent.SetValueAsEnum` (`AIBlueprintHelperLibrary.GetBlackboard` null) (`self.StateKey`) State))

(event `self.ReceiveBeginPlay`
  (bind _blackboardcomponent (`self.UseBlackboard` "/Game/SibJam2/Blueprints/Characters/Bot/BB_Bot.BB_Bot"))
  (`|ExecutionSequence`
    (:`then_0`
      (`BlackboardComponent.SetValueAsObject` _blackboardcomponent (`self.TargetLocKey`) (`self.MoveTarget`)))
    (:`then_1`
      (`BlackboardComponent.SetValueAsObject` _blackboardcomponent (`self.PlayerCharKey`) (`GameplayStatics.GetPlayerCharacter` 0)))))

(fn `UserConstructionScript`)