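; BP_Hold_Sword is a sword pickup that the player can hold, showing the "Поднять" (Pick up) look-at prompt.
; On interaction it disables the sword's collision and passes itself to the player's HoldComponent as the new controlled actor, with ShouldDestroy set.
; SetRarity only stores the rarity; the material lookup by rarity, with a default fallback, is disconnected and never runs.
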(event `self.SetRarity`
  (params (NewRarity :type "Text (by ref)"))
  (set `self.Rarity` NewRarity))

(event `self.InteractWith`
  (params (Caller :type "Actor Object Reference"))
  (`PrimitiveComponent.SetCollisionEnabled` (`self.Sword`) "NoCollision")
  (bind _asbp_player (cast `/Game/SibJam2/Blueprints/Characters/Player/BP_Player` Caller))
  (`SGJ_Player_HoldComponent.SetNewControlledActor` (`/Game/SibJam2/Blueprints/Characters/Player/BP_Player.HoldComponent` _asbp_player) self true))

(fn `GetLookOnMessage`
  (returns (ReturnValue :type Text))
  (return "Поднять"))

(fn `UserConstructionScript`)