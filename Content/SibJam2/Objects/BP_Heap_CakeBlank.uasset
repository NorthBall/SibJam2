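; BP_Heap_CakeBlank displays a countable heap of cake blanks as instances on an InstancedStaticMesh.
; SetHeapCount clears the existing instances and rebuilds the requested number in local space.
; GetTransformByInt places each index on a flat, evenly spaced grid, three across in Y and growing along X, using integer division and modulo.
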(event `self.ReceiveBeginPlay`)

(event `self.SetHeapCount`
  (params (NewCount :type Integer))
  (bind _instancedstaticmesh (`self.InstancedStaticMesh`))
  (`InstancedStaticMeshComponent.ClearInstances` _instancedstaticmesh)
  (for _index (range NewCount)
    (`InstancedStaticMeshComponent.AddInstance` _instancedstaticmesh (`self.GetTransformByInt` _index) false)))

(fn `GetTransformByInt`
  (params (Num :type Integer))
  (returns (Result :type "Transform Structure"))
  (return (`KismetMathLibrary.MakeTransform` (`KismetMathLibrary.MakeVector` (`KismetMathLibrary.Conv_IntToDouble` (* (/ Num 3) 30)) (`KismetMathLibrary.Conv_IntToDouble` (* (mod Num 3) 30))))))

(fn `UserConstructionScript`)