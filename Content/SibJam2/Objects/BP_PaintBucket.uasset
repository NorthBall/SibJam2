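; BP_PaintBucket is an interactable paint bucket that applies its Rarity to the sword a player is holding.
; On BeginPlay it sets the Bucket mesh material by looking up its Rarity as a string key in MaterialMap.
; On interaction it gets the caller's hold component, casts the controlled actor to SGJ_Hold_Sword and calls SetRarity on it.
; Its look-on prompt is a hardcoded Russian string meaning "Paint".
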(event `self.ReceiveBeginPlay`
  (bind (_value _returnvalue) (`BlueprintMapLibrary.Map_Find` (`self.MaterialMap`) (`KismetTextLibrary.Conv_TextToString` (`self.Rarity`))))
  (if _returnvalue
    (`PrimitiveComponent.SetMaterial` (`self.Bucket`) 0 _value)))

(event `self.InteractWith`
  (params (Caller :type "Actor Object Reference"))
  (bind _returnvalue (`self.GetComponentByClass` Caller "/Script/SibJam2.SGJ_Player_HoldComponent"))
  (`/Engine/EditorBlueprintResources/StandardMacros.IsValid` Caller
    (:`Is Valid`
      (`/Engine/EditorBlueprintResources/StandardMacros.IsValid` _returnvalue
        (:`Is Valid`
          (bind _assgj_hold_sword (cast `SGJ_Hold_Sword` (`SGJ_Player_HoldComponent.GetControlledActor` _returnvalue)))
          (`SGJ_Hold_Sword.SetRarity` _assgj_hold_sword (`self.Rarity`)))))))

(fn `GetLookOnMessage`
  (returns (ReturnValue :type Text))
  (return "Покрасить"))

(fn `UserConstructionScript`)