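; BP_Quest_GetFromOutside is a quest type that validates a written quest description before giving it to an adventurer.
; GiveQuestToAdventurer lowercases the text, requires a minimum length, and searches for two occurrences of "трава" (herb), otherwise returning a Russian error message.
; On success it fires OnQuestGivenToAdventurer and notifies the adventurer through a BP_Bot cast, noted as temporary until the bot moves to C++.
; The CalcRealCount event is empty.
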(event `self.CalcRealCount`)

(fn `GiveQuestToAdventurer`
  (params (QuestDescription :type "Text (by ref)"))
  (returns (ErrorDescription :type Text) (ReturnValue :type Boolean))
  (locals (FindPosition :type Integer :default -1) (StringDescription :type String))
  (bind _output_get (set `local.StringDescription` (`KismetStringLibrary.ToLower` (`KismetTextLibrary.Conv_TextToString` QuestDescription))))
  (if (> (`KismetStringLibrary.Len` _output_get) 50)
    (for _ (range 2)
      (bind _output_get_2 (set `local.FindPosition` (`KismetStringLibrary.FindSubstring` (`local.StringDescription`) "трава" false false (`local.FindPosition`))))
      (if (>= _output_get_2 0)
        (`/Engine/EditorBlueprintResources/StandardMacros.IncrementInt` _output_get_2)
        (else
          (return "Нужно упомянуть волшебную траву!" false))))
    (`self.OnQuestGivenToAdventurer`)
    (`/Game/SibJam2/Blueprints/Characters/Bot/BP_Bot.OnQuestGiven` (cast `/Game/SibJam2/Blueprints/Characters/Bot/BP_Bot` (`self.Adventurer`) :!pure true))
    (return "" true)
    (else
      (return "Описание квеста должно быть больше" false))))