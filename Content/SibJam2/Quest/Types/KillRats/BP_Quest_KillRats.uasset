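; BP_Quest_KillRats is a kill-rats quest whose player-written description is validated before it is given to an adventurer.
; GiveQuestToAdventurer requires text over 50 characters, then loops a substring search to confirm three mentions of "крыс" (rats).
; Failures return a Russian error message and false.
; Success fires OnQuestGivenToAdventurer and notifies the adventurer through a BP_Bot cast, noted as temporary until bots move to C++.
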(fn `GiveQuestToAdventurer`
  (params (QuestDescription :type "Text (by ref)"))
  (returns (ErrorDescription :type Text) (ReturnValue :type Boolean))
  (locals (StringDescription :type String) (FindPosition :type Integer :default -1) (ChoosenCount :type Integer))
  (bind _returnvalue (`KismetTextLibrary.Conv_TextToString` QuestDescription))
  (bind _output_get (set `local.StringDescription` _returnvalue))
  (if (> (`KismetStringLibrary.Len` _output_get) 50)
    (for _ (range 3)
      (bind _output_get_2 (set `local.FindPosition` (`KismetStringLibrary.FindSubstring` _returnvalue "крыс" false false (`local.FindPosition`))))
      (if (>= _output_get_2 0)
        (`/Engine/EditorBlueprintResources/StandardMacros.IncrementInt` _output_get_2)
        (else
          (return "Нужно упомянуть крыс 3 раза" false))))
    (`self.OnQuestGivenToAdventurer`)
    (`/Game/SibJam2/Blueprints/Characters/Bot/BP_Bot.OnQuestGiven` (cast `/Game/SibJam2/Blueprints/Characters/Bot/BP_Bot` (`self.Adventurer`) :!pure true))
    (return "" true)
    (else
      (return "Описание квеста должно быть больше" false))))