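; BP_Quest_GetWood is a firewood quest asset that randomizes its task and validates the description given to an adventurer.
; CalcRealCount picks random firewood and cake times plus an even cake count, pushes them to the main GameState's timer and cake heap, and derives the real count from them.
; GiveQuestToAdventurer requires text over 50 characters mentioning firewood ("дров") twice, then notifies the bot or returns a Russian error.
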(event `self.CalcRealCount`
  (set `self.ChosenFirewoodTime` (`KismetArrayLibrary.Array_Random` (`self.PossibleFirewoodTime`)))
  (set `self.ChosenCakeTime` (`KismetArrayLibrary.Array_Random` (`self.PossibleCakeTime`)))
  (bind _output_get (set `self.ChosenCakeNum` (* (`KismetMathLibrary.RandomIntegerInRange` 1 (`self.HalfMaxCake`)) 2)))
  (`|ExecutionSequence`
    (:`then_0`
      (bind _asgsbp_main_state (cast `/Game/SibJam2/Blueprints/StatesAndModes/GSBP_MainState` (`self.GetGameState`)))
      (bind _timerref (`/Game/SibJam2/Blueprints/StatesAndModes/GSBP_MainState.TimerRef` _asgsbp_main_state))
      (set `SGJ_Timer_Watch.TimeForFirewood` (`self.ChosenFirewoodTime`) _timerref)
      (set `SGJ_Timer_Watch.TimeForCake` (`self.ChosenCakeTime`) _timerref)
      (`SGJ_HeapBase.SetHeapCount` (`/Game/SibJam2/Blueprints/StatesAndModes/GSBP_MainState.CakeHeapRef` _asgsbp_main_state) (`self.ChosenCakeNum`)))
    (:`then_1`
      (set `self.RealCount` (/ (* _output_get (`self.ChosenCakeTime`)) (`self.ChosenFirewoodTime`))))))

(fn `GiveQuestToAdventurer`
  (params (QuestDescription :type "Text (by ref)"))
  (returns (ErrorDescription :type Text) (ReturnValue :type Boolean))
  (locals (StringDescription :type String) (FindPosition :type Integer))
  (bind _output_get (set `local.StringDescription` (`KismetStringLibrary.ToLower` (`KismetTextLibrary.Conv_TextToString` QuestDescription))))
  (if (> (`KismetStringLibrary.Len` _output_get) 50)
    (for _ (range 2)
      (bind _output_get_2 (set `local.FindPosition` (`KismetStringLibrary.FindSubstring` _output_get "дров" false false (`local.FindPosition`))))
      (if (>= _output_get_2 0)
        (`/Engine/EditorBlueprintResources/StandardMacros.IncrementInt` _output_get_2)
        (else
          (return "Нужно упомянуть дрова 2раза" false))))
    (`/Game/SibJam2/Blueprints/Characters/Bot/BP_Bot.OnQuestGiven` (cast `/Game/SibJam2/Blueprints/Characters/Bot/BP_Bot` (`self.Adventurer`) :!pure true))
    (return "" true)
    (else
      (return "Описание квеста должно быть больше" false))))