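; Quest payment component that decides what an adventurer demands and whether the caller's held item satisfies it.
; A reroll event randomly requests either gold or a sword of a random rarity from PossibleRarities.
; IsPayAccepted checks the actor in the caller's hold component for a coin or matching-rarity sword, destroys it on success, and returns Russian payment or error text.
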(event `RerollRequestedPay`
  (bind _output_get (set `self.RequestGold` (`KismetMathLibrary.RandomBool`)))
  (if _output_get
    (set `self.RequestedRarity` "")
    (else
      (set `self.RequestedRarity` (`KismetArrayLibrary.Array_Random` (`self.PossibleRarities`))))))

(fn `GetAcceptedPaymentText`
  (returns (PaymentText :type Text))
  (if (`self.RequestGold`)
    (return "")
    (else
      (return (`|FormatText` "Меч {Rarity} (1)" (`self.RequestedRarity`))))))

(fn `GetPayError`
  (returns (TextError :type Text))
  (if (`self.RequestGold`)
    (return "Принеси мне золота!")
    (else
      (return (`|FormatText` "Принеси {Rarity} меч!" (`self.RequestedRarity`))))))

(fn `IsPayAccepted`
  (params (Caller :type "Actor Object Reference"))
  (returns (Result :type Boolean) (TextError :type Text) (TextPayment :type Text))
  (locals (HeldClass :type "Actor Class Reference"))
  (bind _returnvalue (`Actor.GetComponentByClass` Caller "/Script/SibJam2.SGJ_Player_HoldComponent"))
  (bind _returnvalue_2 (`SGJ_Player_HoldComponent.GetControlledActor` _returnvalue))
  (`/Engine/EditorBlueprintResources/StandardMacros.IsValid` Caller
    (:`Is Valid`
      (`/Engine/EditorBlueprintResources/StandardMacros.IsValid` _returnvalue
        (:`Is Valid`
          (`/Engine/EditorBlueprintResources/StandardMacros.IsValid` _returnvalue_2
            (:`Is Valid`
              (if (`self.RequestGold`)
                (if (`KismetMathLibrary.ClassIsChildOf` (`GameplayStatics.GetObjectClass` _returnvalue_2) "/Script/SibJam2.SGJ_HoldCoin")
                  (`SGJ_Player_HoldComponent.SetNewControlledActor` _returnvalue null true)
                  (return true "" (`self.GetAcceptedPaymentText`))
                  (else
                    _))
                (else
                  (bind _assgj_hold_sword (cast `SGJ_Hold_Sword` _returnvalue_2)
                    (:`then`
                      (if (`KismetTextLibrary.EqualEqual_TextText` (`SGJ_Hold_Sword.GetRarity` _assgj_hold_sword) (`self.RequestedRarity`))
                        (`SGJ_Player_HoldComponent.SetNewControlledActor` _returnvalue null true)
                        (return true "" (`self.GetAcceptedPaymentText`))
                        (else
                          _)))
                    (:`CastFailed`
                      _)))))
            (:`Is Not Valid`
              _))
          (return false (`self.GetPayError`) ""))
        (:`Is Not Valid`
          _)))
    (:`Is Not Valid`
      _))
  (return false "Invalid caller" ""))